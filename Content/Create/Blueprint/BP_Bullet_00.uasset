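; Bullet actor that destroys enemies of class BP_Enermy_02 on contact and removes itself two seconds after BeginPlay.
; The Bullet component's hit event checks the other actor's exact class, then passes a DoOnce so each bullet kills at most one enemy.
; A kill destroys the enemy and spawns an actor at the impact location, while the bullet itself persists until its timer ends.
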(event `self.ReceiveBeginPlay`
  (`KismetSystemLibrary.Delay` 2.0)
  (`self.K2_DestroyActor`))

(event `self.Bullet.OnComponentHit`
  (params (HitComponent :type "PrimitiveComponent Object Reference") (OtherActor :type "Actor Object Reference") (OtherComp :type "PrimitiveComponent Object Reference") (NormalImpulse :type "Vector Structure") (Hit :type "HitResult Structure (by ref)"))
  (if (== (`GameplayStatics.GetObjectClass` OtherActor) "/Game/Create/Blueprint/BP_Enermy_02.BP_Enermy_02_C")
    (`/Engine/EditorBlueprintResources/StandardMacros.DoOnce` false
      (:`Completed`
        (`self.K2_DestroyActor` OtherActor)
        (`|SpawnActorFromClass` "/Game/Create/Blueprint/BP_Boom.BP_Boom_C" (`KismetMathLibrary.MakeTransform` (`.Location` (`GameplayStatics.BreakHitResult` Hit))) "Undefined" "MultiplyWithRoot" null null)))))

(fn `UserConstructionScript`)