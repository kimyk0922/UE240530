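; BP_Ele is a trigger actor that shows the WG_Ele UI while something overlaps its Ele_Trigger component.
; Begin overlap creates the widget for player 0, plays its intro animation and, after a short delay, sets mouse cursor visibility from CursorOnOff.
; End overlap hides the cursor, plays the outro animation and, after a delay, removes all widgets, not just this one.
; Overlaps are not filtered by actor, and each one creates a new widget.
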(event `self.Ele_Trigger.OnComponentBeginOverlap`
  (params (OverlappedComponent :type "PrimitiveComponent Object Reference") (OtherActor :type "Actor Object Reference") (OtherComp :type "PrimitiveComponent Object Reference") (OtherBodyIndex :type Integer) (bFromSweep :type Boolean) (SweepResult :type "HitResult Structure (by ref)"))
  (bind _returnvalue (`|CreateWidget` "/Game/Create/Blueprint/WG_Ele.WG_Ele_C" (`GameplayStatics.GetPlayerController` 0)))
  (`UserWidget.AddToViewport` _returnvalue 0)
  (bind _ani_ele_ui_start (`/Game/Create/Blueprint/WG_Ele.Ani_Ele_UI_Start` _returnvalue))
  (`UserWidget.PlayAnimation` _returnvalue _ani_ele_ui_start 0.0 1 "Forward" 1.0 false)
  ;[0.05781 0.1221 0.1746 1 10] Animation_End_line_Settings
  (bind _returnvalue_2 (`MovieSceneSequenceExtensions.GetPlaybackRange` _ani_ele_ui_start))
  (`SequencerScriptingRangeExtensions.GetEndSeconds` _returnvalue_2)
  (`KismetSystemLibrary.Delay` 0.2)
  (set `PlayerController.bShowMouseCursor` (`self.Cursor On/Off`) (`GameplayStatics.GetPlayerController` 0)))

(event `self.Ele_Trigger.OnComponentEndOverlap`
  (params (OverlappedComponent :type "PrimitiveComponent Object Reference") (OtherActor :type "Actor Object Reference") (OtherComp :type "PrimitiveComponent Object Reference") (OtherBodyIndex :type Integer))
  (set `PlayerController.bShowMouseCursor` false (`GameplayStatics.GetPlayerController` 0))
  (`UserWidget.PlayAnimation` (stale `self.Ele_Trigger.OnComponentBeginOverlap` _returnvalue) (`/Game/Create/Blueprint/WG_Ele.Ani_Ele_UI_End` (stale `self.Ele_Trigger.OnComponentBeginOverlap` _returnvalue)) 0.0 1 "Forward" 1.0 false)
  (`KismetSystemLibrary.Delay` 1.0)
  (`WidgetLayoutLibrary.RemoveAllWidgets`))

(fn `UserConstructionScript`)